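; BP_CodeCrystal is a single crystal in a code-entry puzzle, starting dark grey and giving timed color and FMOD sound feedback.
; When hit while Active, it passes its Index to CodeManager and flashes purple with an activation sound if the manager accepts it.
; Show and ShowBad events swap the mesh material to purple or red for a moment, then restore grey.
; Nothing in this Blueprint calls ShowBad.
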(event `self.ReceiveBeginPlay`
  (`PrimitiveComponent.SetMaterial` (`self.StaticMesh`) 0 "/Game/Materials/BasicColours/M_DarkGrey.M_DarkGrey"))

(event `Show`
  (bind _staticmesh (`self.StaticMesh`))
  ;[1 1 1] Flashes purple and then resets
  (`PrimitiveComponent.SetMaterial` _staticmesh 0 "/Game/Materials/Glow/GlowPurple.GlowPurple")
  (`FMODAudioComponent.Play` (`self.FMODActivateCrystal`))
  (`KismetSystemLibrary.Delay` 1.0)
  (`PrimitiveComponent.SetMaterial` _staticmesh 0 "/Game/Materials/BasicColours/M_DarkGrey.M_DarkGrey"))

(event `ShowBad`
  (bind _staticmesh (`self.StaticMesh`))
  ;[1 1 1] Flashes red to show failure
  (`FMODAudioComponent.Play` (`self.FMODCrystalFail`))
  (`PrimitiveComponent.SetMaterial` _staticmesh 0 "/Game/Materials/Glow/EmissiveRed.EmissiveRed")
  (`KismetSystemLibrary.Delay` 1.0)
  (`PrimitiveComponent.SetMaterial` _staticmesh 0 "/Game/Materials/BasicColours/M_DarkGrey.M_DarkGrey"))

(event `/Game/Interfaces/BPI_Hittable.Hit`
  (params (Damage :type "Float (double-precision)") (Hitter :type "Actor Object Reference"))
  ;[1 1 1] Flashes purple when hit if it is the correct entry in the code, notifies the manager it was hit
  (if (`self.active`)
    (bind _success (`/Game/Blueprints/RelicPuzzle2/BP_CodeCrystalManager.CrystalHit` (`self.codeManager`) (`self.index`)))
    (if _success
      (`self.Show`)
      (`FMODAudioComponent.Play` (`self.FMODActivateCrystal`)))))

(fn `UserConstructionScript`)