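; Relic wall torch that lights with a purple flame while its referenced bumper is active, apparently as part of a secret puzzle.
; Tick polls the bumper state and uses LightsON to toggle light, flame visibility and flame material only on changes.
; Each ignition also plays the puzzle-attract FMOD sound on the BP_SecretFoundTrigger found in the level.
; Player-proximity crackle audio logic is disconnected and never runs.
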(event `self.ReceiveTick`
  (params (DeltaSeconds :type "Float (single-precision)"))
  (bind _lightson (`self.LightsON`))
  (if (`/Game/Blueprints/PuzzleObjects/BP_Bumper.Active` (`self.BumperRef`))
    (if (not _lightson)
      (`self.TurnON`)
      (bind _returnvalue (`GameplayStatics.GetActorOfClass` "/Game/Audio/BP/BP_SecretFoundTrigger.BP_SecretFoundTrigger_C"))
      (`FMODAudioComponent.Play` (`/Game/Audio/BP/BP_SecretFoundTrigger.FMODSecretPuzzleAttract` _returnvalue))
      (set `self.LightsON` true))
    (elif _lightson
      (`self.TurnOFF`)
      (set `self.LightsON` false))))

(event `self.Box.OnComponentBeginOverlap`
  (params (OverlappedComponent :type "PrimitiveComponent Object Reference") (OtherActor :type "Actor Object Reference") (OtherComp :type "PrimitiveComponent Object Reference") (OtherBodyIndex :type Integer) (bFromSweep :type Boolean) (SweepResult :type "HitResult Structure (by ref)")))

(event `self.Box.OnComponentEndOverlap`
  (params (OverlappedComponent :type "PrimitiveComponent Object Reference") (OtherActor :type "Actor Object Reference") (OtherComp :type "PrimitiveComponent Object Reference") (OtherBodyIndex :type Integer)))

(event `TurnON`
  (`SceneComponent.SetVisibility` (`self.PointLight`) true false)
  (`SceneComponent.SetVisibility` (`self.Flame`) true false)
  (`PrimitiveComponent.SetMaterial` (`self.Wall_Torch_Test_Model`) 1 "/Game/Materials/Torch/M_TorchFlamePurple.M_TorchFlamePurple")
  (`SceneComponent.SetVisibility` (`self.TorchFire`) true false))

(event `TurnOFF`
  (`SceneComponent.SetVisibility` (`self.PointLight`) false false)
  (`SceneComponent.SetVisibility` (`self.Flame`) false false)
  (`PrimitiveComponent.SetMaterial` (`self.Wall_Torch_Test_Model`) 1 "/Game/Materials/Transparent/M_PRT_TranslucentMaterial.M_PRT_TranslucentMaterial")
  (`SceneComponent.SetVisibility` (`self.TorchFire`) false false))

(fn `UserConstructionScript`)