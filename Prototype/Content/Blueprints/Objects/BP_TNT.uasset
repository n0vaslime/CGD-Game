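; TNT prop that, once activated, simulates physics, ticks and flashes red/white through a countdown scaled by TimeMultiplier, then explodes.
; The blast shakes the camera, spawns BP_Explosion, damages player and enemies in BlastRadius, destroys explodable doors and hits other hittables.
; It also triggers the scripted boulder chase by starting the boulder and boss music and teleporting the hammer button away.
; Afterwards Tick shrinks it to zero scale after a delay instead of destroying it.
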(event `self.ReceiveTick`
  (params (DeltaSeconds :type "Float (single-precision)"))
  (if (`self.destroying`)
    (bind _output_get (set `self.time to destroy` (- (stale _output_get) DeltaSeconds)))
    (if (< _output_get 0.0)
      (`self.SetActorScale3D` (0.0 0.0 0.0)))
    (else
      (`self.updateDetonation` DeltaSeconds))))

(event `/Game/Interfaces/BPI_Activateable.Activate`
  (`self.startDetonation`))

(event `/Game/Interfaces/BPI_Activateable.Deactivate`
  (set `self.meaningless` true))

(fn `explode`
  (bind (_returnvalue_location _returnvalue_rotation) (`KismetMathLibrary.BreakTransform` (`self.GetTransform`)))
  (bind _blast_radius (`self.blast_radius`))
  (bind _blast_damage (`self.blast_damage`))
  ;[1 1 1] Play Boulder Rolling
  (bind _returnvalue (`GameplayStatics.GetActorOfClass` "/Game/Blueprints/BoulderChase/BP_ChaseBoulder.BP_ChaseBoulder_C"))
  (`FMODAudioComponent.Play` (`/Game/Blueprints/BoulderChase/BP_ChaseBoulder.FMODBoulderRolling` _returnvalue))
  ;[1 1 1] Play Boss Music
  (bind _returnvalue_2 (`GameplayStatics.GetActorOfClass` "/Game/Audio/BP/BP_MusicFinal1.BP_MusicFinal1_C"))
  (`/Game/Audio/BP/BP_MusicFinal1.StartBossDrop` _returnvalue_2)
  ;[1 1 1] Explode SFX & Stop Ticking
  (`FMODAudioComponent.Stop` (`self.FMODClock`))
  (`FMODAudioComponent.Play` (`self.FMODExplosion`))
  ;[1 1 1] camera shake
  (bind _asbp_third_person_character (cast `/Game/ThirdPerson/Blueprints/BP_ThirdPersonCharacter` (`GameplayStatics.GetPlayerCharacter` 0)))
  (`GameplayStatics.PlayWorldCameraShake` "/Game/Blueprints/CameraShake/BP_TNTCameraShake.BP_TNTCameraShake_C" (`SceneComponent.K2_GetComponentLocation` (`/Game/ThirdPerson/Blueprints/BP_ThirdPersonCharacter.FollowCamera` _asbp_third_person_character)) 0.0 100.0 1.0 true)
  (`|SpawnActorFromClass` "/Game/Blueprints/Objects/BP_Explosion.BP_Explosion_C" (`KismetMathLibrary.MakeTransform` _returnvalue_location _returnvalue_rotation (`KismetMathLibrary.Conv_DoubleToVector` (/ (`SphereComponent.GetScaledSphereRadius` _blast_radius) 50.0))) "Undefined" "MultiplyWithRoot" null null)
  (for _array_element (`PrimitiveComponent.GetOverlappingActors` _blast_radius null)
    (bind _asbp_third_person_character_2 (cast `/Game/ThirdPerson/Blueprints/BP_ThirdPersonCharacter` _array_element)
      (:`then`
        (`/Game/ThirdPerson/Blueprints/BP_ThirdPersonCharacter.takeDamage` _asbp_third_person_character_2 _blast_damage))
      (:`CastFailed`
        (bind _asbp_enemy_parent (cast `/Game/Blueprints/Enemies/BP_EnemyParent` _array_element)
          (:`then`
            (`/Game/Blueprints/Enemies/BP_EnemyParent.takeDamage` _asbp_enemy_parent _blast_damage))
          (:`CastFailed`
            (if (`KismetMathLibrary.ClassIsChildOf` (`GameplayStatics.GetObjectClass` _array_element) "/Game/Blueprints/Objects/BP_ExplodableDoor.BP_ExplodableDoor_C")
              (`self.K2_DestroyActor` _array_element)
              (else
                (bind _asbpi_hittable (cast `/Game/Interfaces/BPI_Hittable` _array_element))
                (`/Game/Interfaces/BPI_Hittable.Hit` _asbpi_hittable 0.0 self))))))))
  (set `self.destroying` true)
  (`PrimitiveComponent.SetSimulatePhysics` (`self.TNT`) false)
  (bind _returnvalue_3 (`GameplayStatics.GetActorOfClass` "/Game/Blueprints/PuzzleObjects/BP_HammerButton.BP_HammerButton_C"))
  (`self.K2_SetActorLocation` _returnvalue_3 (1000000.0 0.0 -100000.0) false false)
  (bind _returnvalue_4 (`GameplayStatics.GetActorOfClass` "/Game/Blueprints/BoulderChase/BP_ChaseBoulder.BP_ChaseBoulder_C"))
  (set `/Game/Blueprints/BoulderChase/BP_ChaseBoulder.Active` true _returnvalue_4))

(fn `Get Reinforced`
  (returns (value :type Boolean))
  (return true))

(fn `startDetonation`
  (set `self.detonating` true)
  (`PrimitiveComponent.SetSimulatePhysics` (`self.TNT`) true)
  (`FMODAudioComponent.Play` (`self.FMODClock`)))

(fn `updateDetonation`
  (params (`Delta Seconds` :type "Float (double-precision)"))
  (if (`self.detonating`)
    (`self.updateFlash` `Delta Seconds`)
    (bind _output_get (set `self.detonation_timer` (- (`self.detonation_timer`) (/ `Delta Seconds` (`self.time_multiplier`)))))
    (`/Engine/EditorBlueprintResources/StandardMacros.CompareFloat` _output_get
      (:`==`
        _)
      (:`<`
        _))
    (`self.explode`)))

(fn `updateFlash`
  (params (`Delta Seconds` :type "Float (double-precision)"))
  (bind _tnt (`self.TNT`))
  (bind _output_get (set `self.flash_timer` (- (`self.flash_timer`) (/ `Delta Seconds` (`self.time_multiplier`)))))
  (`/Engine/EditorBlueprintResources/StandardMacros.CompareFloat` _output_get
    (:`==`
      _)
    (:`<`
      _))
  (if (== (`PrimitiveComponent.GetMaterial` _tnt 0) "/Game/Materials/BasicColours/M_Red.M_Red")
    (`PrimitiveComponent.SetMaterial` _tnt 0 "/Game/Materials/BasicColours/M_White.M_White")
    (else
      (`PrimitiveComponent.SetMaterial` _tnt 0 "/Game/Materials/BasicColours/M_Red.M_Red")))
  (set `self.flash_timer` (`self.flash_timer_max`)))

(fn `UserConstructionScript`)