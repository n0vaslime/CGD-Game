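; BP_RoomTorch is a wall torch with a flame material, fire effect, point light and FMOD crackle sound.
; Extinguish swaps the flame material to coal, deactivates the fire, hides the light and stops the crackle.
; ResetTorch restores all four unless PermanentlyExtinguished is set.
; The Box overlap events do nothing, as their logic to play and stop the crackle is disconnected.
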(event `self.Box.OnComponentBeginOverlap`
  (params (OverlappedComponent :type "PrimitiveComponent Object Reference") (OtherActor :type "Actor Object Reference") (OtherComp :type "PrimitiveComponent Object Reference") (OtherBodyIndex :type Integer) (bFromSweep :type Boolean) (SweepResult :type "HitResult Structure (by ref)")))

(event `self.Box.OnComponentEndOverlap`
  (params (OverlappedComponent :type "PrimitiveComponent Object Reference") (OtherActor :type "Actor Object Reference") (OtherComp :type "PrimitiveComponent Object Reference") (OtherBodyIndex :type Integer)))

(fn `extinguish`
  (`PrimitiveComponent.SetMaterial` (`self.Wall_Torch_Test_Model`) 1 "/Game/ART+VISUALS/Materials+Textures/Torch/Coal/Coal.Coal")
  (`ActorComponent.Deactivate` (`self.TorchFire`))
  (`SceneComponent.SetVisibility` (`self.PointLight`) false false)
  (`FMODAudioComponent.Stop` (`self.FMODCrackle`)))

(fn `resetTorch`
  (if (not (`self.permanently_extinguished`))
    (`PrimitiveComponent.SetMaterial` (`self.Wall_Torch_Test_Model`) 1 "/Game/Materials/Torch/M_TorchFlame.M_TorchFlame")
    (`ActorComponent.Activate` (`self.TorchFire`) true)
    (`SceneComponent.SetVisibility` (`self.PointLight`) true false)
    (`FMODAudioComponent.Play` (`self.FMODCrackle`))))

(fn `UserConstructionScript`)