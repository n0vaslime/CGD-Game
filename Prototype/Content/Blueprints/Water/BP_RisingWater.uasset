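; Rising water actor that moves its Water component from a Start point to an End point when activated.
; BeginPlay snaps Water to Start and sets the timeline's play rate to the inverse of PlatformPlayRate, so larger values mean slower movement.
; The Activate event plays the timeline, whose alpha interpolates the world location between the two markers without sweeping.
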(event `self.ReceiveBeginPlay`
  ;[1 1 1] Set Start Position & Speed
  (`SceneComponent.K2_SetWorldLocation` (`self.Water`) (`SceneComponent.K2_GetComponentLocation` (`self.Start`)) false false)
  (`TimelineComponent.SetPlayRate` (`self.PlatformMovementTimeline`) (/ 1.0 (`self.PlatformPlayRate`))))

(event `/Game/Interfaces/BPI_Activateable.Activate`
  ;[1 1 1] Activated Platform Movement
  (bind (_direction _alpha) (`Timeline|PlatformMovementTimeline`)
    (:`Update`
      (`SceneComponent.K2_SetWorldLocation` (`self.Water`) (`KismetMathLibrary.VLerp` (`SceneComponent.K2_GetComponentLocation` (`self.Start`)) (`SceneComponent.K2_GetComponentLocation` (`self.End`)) _alpha) false false))))

(fn `UserConstructionScript`)