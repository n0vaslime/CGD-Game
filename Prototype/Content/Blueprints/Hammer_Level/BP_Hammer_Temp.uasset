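; Temporary hammer actor that flies forward, returns to the player and carries a colour shown on its head.
; Tick moves it along local X while Moving, or eases it horizontally toward RetrieveTargetLocation while Retrieving.
; Any overlap stops it: the player picks it up via BP_Hammer_Interaction, while other non-AoE actors trigger a coloured BP_HammerAoE and reset it to White.
; UpdateColour swaps the head material, with Yellow and Green materials left unassigned.
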(event `self.ReceiveActorBeginOverlap`
  (params (OtherActor :type "Actor Object Reference"))
  (bind (_returnvalue_location _returnvalue_rotation _returnvalue_scale) (`KismetMathLibrary.BreakTransform` (`self.GetTransform`)))
  (set `self.Retrieving` false)
  (set `self.Moving` false)
  (bind _asbp_third_person_character (cast `/Game/ThirdPerson/Blueprints/BP_ThirdPersonCharacter` OtherActor)
    (:`then`
      ;[0 0 0] Picks up Hammer if it collides with Player
      (`/Game/Blueprints/Hammer_Level/BP_Hammer_Interaction.PickUpHammer` (`self.GetComponentByClass` _asbp_third_person_character "/Game/Blueprints/Hammer_Level/BP_Hammer_Interaction.BP_Hammer_Interaction_C") self))
    (:`CastFailed`
      (cast `/Game/Blueprints/Hammer_Level/BP_HammerAoE` OtherActor
        (:`CastFailed`
          ;[0 0 0] Generates AOE if it collides with something other than the Player AND if it has a colour. If it has no colour (White by default), there is no AOE.
          (if (!= (`self.Colour`) 0)
            (`|SpawnActorFromClass` "/Game/Blueprints/Hammer_Level/BP_HammerAoE.BP_HammerAoE_C" (`KismetMathLibrary.MakeTransform` (+ _returnvalue_location (0.0 0.0 50.0)) _returnvalue_rotation _returnvalue_scale) "AlwaysSpawn" "MultiplyWithRoot" null (`self.Colour`) null)
            (`self.Update Colour` "NewEnumerator0")))))))

(event `self.ReceiveTick`
  (params (DeltaSeconds :type "Float (single-precision)"))
  (bind _returnvalue (`self.GetTransform`))
  (bind (_retrievetargetlocation_x _retrievetargetlocation_y) (`KismetMathLibrary.BreakVector` (`self.RetrieveTargetLocation`)))
  ;[0 0 0] Moves the Object if Moving Bool is True
  (if (`self.Moving`)
    (`self.K2_AddActorLocalOffset` (`KismetMathLibrary.MakeVector` (* DeltaSeconds (`self.Speed`))))
    (else
      ;[0 0 0] Retrieves Hammer. Moves in straight line towards Player
      (if (`self.Retrieving`)
        (`self.K2_AddActorWorldTransform` (`KismetMathLibrary.MakeTransform` (* (- (`KismetMathLibrary.MakeVector` _retrievetargetlocation_x _retrievetargetlocation_y) (`KismetMathLibrary.MakeVector` (.x (.location _returnvalue)) (.y (.location _returnvalue)))) DeltaSeconds)))))))

(event `Update Colour`
  (params (`New Colour` :type "/Game/Enums/ENUM_Colours Enum" :default "NewEnumerator0"))
  ;[0 0 0] Updates Colour of Hammer Head when called
  (bind _output_get (set `self.Colour` `New Colour`))
  (switch `/Game/Enums/ENUM_Colours` _output_get
    (:`NewEnumerator0`
      (`PrimitiveComponent.SetMaterial` (`self.Head`) 0 "/Game/Materials/BasicColours/M_White.M_White"))
    (:`NewEnumerator1`
      (`PrimitiveComponent.SetMaterial` (`self.Head`) 0 "/Game/Materials/BasicColours/M_Red.M_Red"))
    (:`NewEnumerator2`
      (`PrimitiveComponent.SetMaterial` (`self.Head`) 0 "/Game/Materials/BasicColours/M_Blue.M_Blue"))
    (:`NewEnumerator3`
      (`PrimitiveComponent.SetMaterial` (`self.Head`) 0 null))
    (:`NewEnumerator4`
      (`PrimitiveComponent.SetMaterial` (`self.Head`) 0 null))))

(fn `UserConstructionScript`)