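; BP_ExamineObject is a component that lets the player examine its owning object up close through a camera.
; Tick checks player distance, enabling examination and applying a red glow overlay to the owner's static meshes when nearby.
; Examine toggles a timed view blend between character and Camera, disabling movement and glow while zoomed in.
; A CameraMoving flag ignores further Examine calls until each blend finishes.
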(event `self.ReceiveBeginPlay`
  (bind _asbp_third_person_character (cast `/Game/ThirdPerson/Blueprints/BP_ThirdPersonCharacter` (`GameplayStatics.GetPlayerCharacter` 0)))
  (set `self.As BP Third Person Character` _asbp_third_person_character))

(event `self.ReceiveTick`
  (params (DeltaSeconds :type "Float (single-precision)"))
  ;[0 0 0] Less than 1000 units away from Player
  (if (< (`KismetMathLibrary.Vector_Distance` (`Actor.K2_GetActorLocation` (`self.As BP Third Person Character`)) (`Actor.K2_GetActorLocation` (`self.GetOwner`))) 250.0)
    ;[0 0 0] Disables effect if currently examining object
    (set `self.CanExamine` true)
    (if (`self.DisplayEffect`)
      ;[0 0 0] Enables mesh overlay
      (for _array_element (`Actor.K2_GetComponentsByClass` (`self.GetOwner`) "/Script/Engine.StaticMeshComponent")
        (`MeshComponent.SetOverlayMaterial` _array_element "/Game/Materials/Glow/GlowRed.GlowRed"))
      (else
        ;[0 0 0] Does not render mesh overlay
        (for _array_element_2 (`Actor.K2_GetComponentsByClass` (`self.GetOwner`) "/Script/Engine.StaticMeshComponent") :!label _label
          (`MeshComponent.SetOverlayMaterial` _array_element_2 null))))
    (else
      (set `self.CanExamine` false)
      (goto _label))))

(event `Examine`
  (if (`self.CameraMoving`)
    _
    (elif (`self.CanExamine`)
      (if (`self.Examining`)
        ;[0 0 0] Zooms out
        (set `self.Examining` false)
        (set `self.DisplayEffect` true)
        (`PlayerController.SetViewTargetWithBlend` (`GameplayStatics.GetPlayerController` 0) (`self.As BP Third Person Character`) 1.0 "VTBlend_Linear" 0.0 false)
        (set `self.CameraMoving` true)
        (`KismetSystemLibrary.Delay` 1.0)
        (set `self.CameraMoving` false)
        (`CharacterMovementComponent.SetMovementMode` (`Character.CharacterMovement` (`self.As BP Third Person Character`)) "MOVE_Walking" 0)
        (else
          ;[0 0 0] Zooms in
          (set `self.Examining` true)
          (set `self.DisplayEffect` false)
          (`CharacterMovementComponent.SetMovementMode` (`Character.CharacterMovement` (`self.As BP Third Person Character`)) "MOVE_None" 0)
          (`PlayerController.SetViewTargetWithBlend` (`GameplayStatics.GetPlayerController` 0) (`self.Camera`) 1.0 "VTBlend_Linear" 0.0 false)
          (set `self.CameraMoving` true)
          (`KismetSystemLibrary.Delay` 1.0)
          (set `self.CameraMoving` false))))))