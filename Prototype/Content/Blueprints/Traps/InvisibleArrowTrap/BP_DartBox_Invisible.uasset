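; Dart dispenser trap that fires poison darts and can switch between visible and invisible states.
; Trigger, gated by CanShoot, waits briefly, spawns a dart at the PoisonDartDirection transform, passes it the box's visibility and ownership, and plays an FMOD sound.
; Activate makes the block's orange material transparent and clears Visible; Deactivate restores both.
; When firing while invisible, a DartShake timeline wobbles the block's rotation.
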(event `self.Trigger`
  (bind _poisondartdirection (`self.PoisonDartDirection`))
  (bind (_returnvalue_location _returnvalue_rotation _returnvalue_scale) (`KismetMathLibrary.BreakTransform` (`SceneComponent.GetRelativeTransform` (`self.DispenserBlock`))))
  (if (`self.CanShoot`)
    (`KismetSystemLibrary.Delay` 0.1)
    (`|ExecutionSequence`
      (:`then_0`
        (bind _returnvalue (`|SpawnActorFromClass` "/Game/Blueprints/Traps/InvisibleArrowTrap/BP_PoisonDart_Invisible.BP_PoisonDart_Invisible_C" (`KismetMathLibrary.MakeTransform` (`SceneComponent.K2_GetComponentLocation` _poisondartdirection) (`SceneComponent.K2_GetComponentRotation` _poisondartdirection)) "Undefined" "MultiplyWithRoot" self null))
        (`/Game/Blueprints/Traps/InvisibleArrowTrap/BP_PoisonDart_Invisible.Show` _returnvalue (`self.Visible`))
        (`FMODAudioComponent.Play` (`self.FMODDartSound`))
        (set `/Game/Blueprints/Traps/Dart_Trap/BP_PoisonDart.OwningDartBox` self _returnvalue))
      (:`then_1`
        (if (not (`self.Visible`))
          (bind (_direction _newtrack_0) (`Timeline|DartShake` :!label _label)
            (:`Update`
              (`SceneComponent.K2_SetRelativeTransform` (`self.DispenserBlock`) (`KismetMathLibrary.MakeTransform` _returnvalue_location (`KismetMathLibrary.MakeRotator` _newtrack_0 _newtrack_0 _newtrack_0) _returnvalue_scale) false false))
            (:`Finished`
              (goto _label :!via `SetNewTime`))))))))

(event `/Game/Interfaces/BPI_Activateable.Activate`
  (`PrimitiveComponent.SetMaterial` (`self.DispenserBlock`) 1 "/Game/Materials/Transparent/MI_Orange_Transparent.MI_Orange_Transparent")
  (set `self.Visible` false))

(event `/Game/Interfaces/BPI_Activateable.Deactivate`
  (`PrimitiveComponent.SetMaterial` (`self.DispenserBlock`) 1 "/Game/Materials/Shaders/M_EmissiveOrange.M_EmissiveOrange")
  (set `self.Visible` true))

(fn `UserConstructionScript`
  (`parent.UserConstructionScript`))