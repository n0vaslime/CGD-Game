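; Poison dart variant for the invisible arrow trap that can switch between a revealed, active state and a hidden, inactive one.
; Its Show event swaps both dart material slots between solid materials and a transparent orange one.
; The same event enables query-only collision on the player detection collider when shown and disables it when hidden.
; BeginPlay, Tick and construction only defer to the parent class.
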(event `self.ReceiveBeginPlay`
  (`parent.ReceiveBeginPlay`))

(event `self.ReceiveTick`
  (params (DeltaSeconds :type "Float (single-precision)"))
  (`parent.ReceiveTick` DeltaSeconds))

(event `Show`
  (params (Show :type Boolean))
  (bind _poison_dart (`self.Poison_Dart`))
  (bind _playerdetectcollidor (`self.PlayerDetectCollidor`))
  (if Show
    (`PrimitiveComponent.SetMaterial` _poison_dart 0 "/Game/Materials/Shaders/M_EmissiveOrange.M_EmissiveOrange")
    (`PrimitiveComponent.SetMaterial` _poison_dart 1 "/Game/Materials/ClayMaterials/MI_ClayGreen.MI_ClayGreen")
    (`PrimitiveComponent.SetCollisionEnabled` _playerdetectcollidor "QueryOnly")
    (else
      (`PrimitiveComponent.SetMaterial` _poison_dart 0 "/Game/Materials/Transparent/MI_Orange_Transparent.MI_Orange_Transparent")
      (`PrimitiveComponent.SetMaterial` _poison_dart 1 "/Game/Materials/Transparent/MI_Orange_Transparent.MI_Orange_Transparent")
      (`PrimitiveComponent.SetCollisionEnabled` _playerdetectcollidor "NoCollision"))))

(fn `UserConstructionScript`
  (`parent.UserConstructionScript`))