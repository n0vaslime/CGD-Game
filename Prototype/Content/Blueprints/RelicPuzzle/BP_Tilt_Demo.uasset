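; Tilt puzzle demo in the relic puzzle set, with tagged platform pieces and trigger volumes that respond to BP_Disc.
; BeginPlay raises DefaultShow children of Platform, while Lvl1 and Lvl2 events, not called here, raise or lower pieces by tag.
; The two level triggers destroy themselves and activate their side doors on disc overlap.
; The completion trigger reactivates SideDoor1 on any overlap, then destroys the actor after a delay.
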(event `self.ReceiveTick`
  (params (DeltaSeconds :type "Float (single-precision)")))

(event `self.ReceiveBeginPlay`
  (`self.DefaultLvl`))

(event `DefaultLvl`
  (for _array_element (`SceneComponent.GetChildrenComponents` (`self.Platform`) false)
    (if (`ActorComponent.ComponentHasTag` _array_element "DefaultShow")
      (bind (_relativelocation_x _relativelocation_y) (`KismetMathLibrary.BreakVector` (`SceneComponent.RelativeLocation` _array_element)))
      (`SceneComponent.K2_SetRelativeLocation` _array_element (`KismetMathLibrary.MakeVector` _relativelocation_x _relativelocation_y 100.0) false false))))

(event `Lvl1`
  (for _array_element (`SceneComponent.GetChildrenComponents` (`self.Platform`) false)
    (if (`ActorComponent.ComponentHasTag` _array_element "ShowLvl1")
      (bind (_relativelocation_x _relativelocation_y) (`KismetMathLibrary.BreakVector` (`SceneComponent.RelativeLocation` _array_element)))
      (`SceneComponent.K2_SetRelativeLocation` _array_element (`KismetMathLibrary.MakeVector` _relativelocation_x _relativelocation_y 100.0) false false)
      (elif (`ActorComponent.ComponentHasTag` _array_element "HideLvl1")
        (`SceneComponent.K2_SetRelativeLocation` _array_element (`KismetMathLibrary.MakeVector` _relativelocation_x _relativelocation_y) false false)))))

(event `Lvl2`
  (for _array_element (`SceneComponent.GetChildrenComponents` (`self.Platform`) false)
    (if (`ActorComponent.ComponentHasTag` _array_element "ShowLvl2")
      (bind (_relativelocation_x _relativelocation_y) (`KismetMathLibrary.BreakVector` (`SceneComponent.RelativeLocation` _array_element)))
      (`SceneComponent.K2_SetRelativeLocation` _array_element (`KismetMathLibrary.MakeVector` _relativelocation_x _relativelocation_y 100.0) false false)
      (elif (`ActorComponent.ComponentHasTag` _array_element "HideLvl2")
        (`SceneComponent.K2_SetRelativeLocation` _array_element (`KismetMathLibrary.MakeVector` _relativelocation_x _relativelocation_y) false false)))))

(event `self.TriggerLvl1.OnComponentBeginOverlap`
  (params (OverlappedComponent :type "PrimitiveComponent Object Reference") (OtherActor :type "Actor Object Reference") (OtherComp :type "PrimitiveComponent Object Reference") (OtherBodyIndex :type Integer) (bFromSweep :type Boolean) (SweepResult :type "HitResult Structure (by ref)"))
  (if (`GameplayStatics.ObjectIsA` OtherActor "/Game/Blueprints/RelicPuzzle/BP_Disc.BP_Disc_C")
    (`GameplayStatics.GetActorOfClass` "/Game/Blueprints/RelicPuzzle/BP_Disc.BP_Disc_C")
    (`ActorComponent.K2_DestroyComponent` (`self.TriggerLvl1`))
    (`/Game/Interfaces/BPI_Activateable.Activate` (`self.SideDoor1`))))

(event `self.TriggerLvl2.OnComponentBeginOverlap`
  (params (OverlappedComponent :type "PrimitiveComponent Object Reference") (OtherActor :type "Actor Object Reference") (OtherComp :type "PrimitiveComponent Object Reference") (OtherBodyIndex :type Integer) (bFromSweep :type Boolean) (SweepResult :type "HitResult Structure (by ref)"))
  (if (`GameplayStatics.ObjectIsA` OtherActor "/Game/Blueprints/RelicPuzzle/BP_Disc.BP_Disc_C")
    (`GameplayStatics.GetActorOfClass` "/Game/Blueprints/RelicPuzzle/BP_Disc.BP_Disc_C")
    (`ActorComponent.K2_DestroyComponent` (`self.TriggerLvl2`))
    (`/Game/Interfaces/BPI_Activateable.Activate` (`self.SideDoor2`))))

(event `self.TriggerComplete.OnComponentBeginOverlap`
  (params (OverlappedComponent :type "PrimitiveComponent Object Reference") (OtherActor :type "Actor Object Reference") (OtherComp :type "PrimitiveComponent Object Reference") (OtherBodyIndex :type Integer) (bFromSweep :type Boolean) (SweepResult :type "HitResult Structure (by ref)"))
  (if (`GameplayStatics.ObjectIsA` OtherActor "/Game/Blueprints/RelicPuzzle/BP_Disc.BP_Disc_C")
    _
    (else
      _))
  (`/Game/Interfaces/BPI_Activateable.Activate` (`self.SideDoor1`))
  (`ActorComponent.K2_DestroyComponent` (`self.TriggerComplete`))
  (`KismetSystemLibrary.Delay` 2.5)
  (`self.K2_DestroyActor`))

(fn `UserConstructionScript`)