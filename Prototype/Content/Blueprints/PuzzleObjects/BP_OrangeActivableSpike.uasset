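; BP_OrangeActivableSpike is an orange spike puzzle hazard that can be switched between shown and hidden states.
; Show and Hide swap the orange transparent material on the spikes and their box, toggle the box collision between query-only and none, and set a Shown flag.
; The HitObject override forwards hits to the parent's logic only while the spike is shown.
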(event `/Game/Interfaces/BPI_Showable.show`
  (params (crystal_id :type Integer))
  (bind _spikebox (`self.SpikeBox`))
  (`PrimitiveComponent.SetMaterial` _spikebox 0 "/Game/Materials/Transparent/MI_Orange_Transparent_2.MI_Orange_Transparent_2")
  (`PrimitiveComponent.SetMaterial` (`self.Spikes`) 0 "/Game/Materials/Transparent/MI_Orange_Transparent_2.MI_Orange_Transparent_2")
  (`PrimitiveComponent.SetCollisionEnabled` _spikebox "QueryOnly")
  (set `self.shown` true))

(event `/Game/Interfaces/BPI_Showable.hide`
  (params (crystal_id :type Integer))
  (`PrimitiveComponent.SetMaterial` (`self.Spikes`) 0 "/Game/Materials/Transparent/MI_Orange_Transparent.MI_Orange_Transparent")
  (`PrimitiveComponent.SetMaterial` (`self.SpikeBox`) 0 "/Game/Materials/Transparent/MI_Orange_Transparent.MI_Orange_Transparent")
  (`PrimitiveComponent.SetCollisionEnabled` (`self.SpikeBox`) "NoCollision")
  (set `self.shown` false))

(fn `hitObject`
  (params (hit_actor :type "Actor Object Reference") (hit_component :type "PrimitiveComponent Object Reference"))
  (if (`self.shown`)
    (`parent.hitObject` hit_actor hit_component)))

(fn `UserConstructionScript`
  (`parent.UserConstructionScript`))