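; Blueprint for a blue key pickup used in puzzles.
; When BP_ThirdPersonCharacter overlaps its trigger while the key is available, it sets the character's HasBlueKey flag and plays that character's FMOD key-found sound.
; CollectedKey then marks it unavailable, hides the mesh and disables its collision.
; ResetKey makes it available and visible again but leaves mesh collision unchanged.
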(event `self.trigger.OnComponentBeginOverlap`
  (params (OverlappedComponent :type "PrimitiveComponent Object Reference") (OtherActor :type "Actor Object Reference") (OtherComp :type "PrimitiveComponent Object Reference") (OtherBodyIndex :type Integer) (bFromSweep :type Boolean) (SweepResult :type "HitResult Structure (by ref)"))
  (if (`self.is_available`)
    (bind _asbp_third_person_character (cast `/Game/ThirdPerson/Blueprints/BP_ThirdPersonCharacter` OtherActor))
    (set `/Game/ThirdPerson/Blueprints/BP_ThirdPersonCharacter.HasBlueKey` true _asbp_third_person_character)
    (`FMODAudioComponent.Play` (`/Game/ThirdPerson/Blueprints/BP_ThirdPersonCharacter.FMODkeyFound` _asbp_third_person_character))
    (`self.collectedKey`)))

(fn `collectedKey`
  (bind _staticmesh (`self.StaticMesh`))
  (set `self.is_available` false)
  (`SceneComponent.SetVisibility` _staticmesh false false)
  (`PrimitiveComponent.SetCollisionEnabled` _staticmesh "NoCollision"))

(fn `resetKey`
  (set `self.is_available` true)
  (`SceneComponent.SetVisibility` (`self.StaticMesh`) true false))

(fn `UserConstructionScript`)