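; BP_OrangeCrystal is a puzzle crystal that toggles on each Hit, showing or hiding linked objects and playing an FMOD sound.
; Activation first calls deactivate on all orange crystals in the level, so only one stays active.
; Both states swap between emissive and dark orange materials and call Show or Hide on ObjectToShow entries through BPI_Showable.
; OpenDoor is an empty stub.
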(event `self.Hit`
  (params (Damage :type "Float (double-precision)") (Hitter :type "Actor Object Reference"))
  (if (`self.Activated`)
    (`self.deactivateCrystal`)
    (`FMODAudioComponent.Play` (`self.FMODCrystalActivation`))
    (else
      (`self.activateCrystal`)
      (`FMODAudioComponent.Play` (`self.FMODCrystalActivation`)))))

(fn `activateCrystal`
  (bind _outactors (`GameplayStatics.GetAllActorsOfClass` "BP_OrangeCrystal_C"))
  (`self.deactivateCrystal` _outactors)
  (`PrimitiveComponent.SetMaterial` (`self.CrystalMesh`) 0 "/Game/Materials/Shaders/M_EmissiveOrange.M_EmissiveOrange")
  (for _array_element (`self.ObjectToShow`)
    (bind _asbpi_showable (cast `/Game/Interfaces/BPI_Showable` _array_element))
    (`/Game/Interfaces/BPI_Showable.show` _asbpi_showable 0))
  (set `self.Activated` true))

(fn `deactivateCrystal`
  (`PrimitiveComponent.SetMaterial` (`self.CrystalMesh`) 0 "/Game/Materials/BasicColours/M_DarkOrange.M_DarkOrange")
  (for _array_element (`self.ObjectToShow`)
    (bind _asbpi_showable (cast `/Game/Interfaces/BPI_Showable` _array_element))
    (`/Game/Interfaces/BPI_Showable.hide` _asbpi_showable 0))
  (set `self.Activated` false))

(fn `OpenDoor`)

(fn `UserConstructionScript`)