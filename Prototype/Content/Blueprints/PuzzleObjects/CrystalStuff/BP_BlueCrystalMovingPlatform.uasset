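; Blue crystal variant of a moving platform puzzle object, with three visual states: shown, hidden and partially hidden.
; Show and PartiallyHide make the Platform component visible and swap its material between two blue translucent looks, while Hide turns visibility off.
; These events change only visibility and material, leaving collision untouched.
; The file contains no movement logic and no callers for the three events.
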(event `/Game/Interfaces/BPI_Showable.show`
  (params (crystal_id :type Integer))
  (bind _platform (`self.platform`))
  (`SceneComponent.SetVisibility` _platform true false)
  (`PrimitiveComponent.SetMaterial` _platform 0 "/Game/Materials/Transparent/MI_TranslucentBlue.MI_TranslucentBlue"))

(event `/Game/Interfaces/BPI_Showable.hide`
  (params (crystal_id :type Integer))
  (`SceneComponent.SetVisibility` (`self.platform`) false false))

(event `/Game/Interfaces/BPI_Showable.partiallyHide`
  (params (crystal_id :type Integer))
  (bind _platform (`self.platform`))
  (`SceneComponent.SetVisibility` _platform true false)
  (`PrimitiveComponent.SetMaterial` _platform 0 "/Game/Materials/Transparent/MI_Blue_Transparent_2.MI_Blue_Transparent_2"))

(fn `UserConstructionScript`
  (`parent.UserConstructionScript`))