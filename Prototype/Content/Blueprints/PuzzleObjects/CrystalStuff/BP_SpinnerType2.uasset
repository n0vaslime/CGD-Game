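; Crystal puzzle spinner that shows, fades or hides its removed blue cylinder segment in response to crystal events.
; Show stores any positive crystal ID, reveals the segment in translucent blue and plays the activation sound if not already lit.
; PartiallyHide and Hide act only for the stored ID: one swaps material and plays a deactivation sound once, the other hides the segment and resets both state flags.
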(event `/Game/Interfaces/BPI_Showable.show`
  (params (crystal_id :type Integer))
  (bind _blue_cylinder_removed_segment (`self.blue_cylinder_removed_segment`))
  (if (> crystal_id 0)
    (set `self.crystal_id_to_hide_this` crystal_id))
  (`SceneComponent.SetVisibility` _blue_cylinder_removed_segment true false)
  (`PrimitiveComponent.SetMaterial` _blue_cylinder_removed_segment 0 "/Game/Materials/Transparent/MI_TranslucentBlue.MI_TranslucentBlue")
  (if (not (`self.IsLit`))
    (`FMODAudioComponent.Play` (`self.FMODActivateBlueCrystal`))
    (set `self.IsLit` true)))

(event `/Game/Interfaces/BPI_Showable.hide`
  (params (crystal_id :type Integer))
  (`/Engine/EditorBlueprintResources/StandardMacros.CompareInt` crystal_id (`self.crystal_id_to_hide_this`)
    (:`==`
      (`SceneComponent.SetVisibility` (`self.blue_cylinder_removed_segment`) false false)
      (set `self.IsLit` false)
      (set `self.IsFlashing` false))))

(event `/Game/Interfaces/BPI_Showable.partiallyHide`
  (params (crystal_id :type Integer))
  (bind _blue_cylinder_removed_segment (`self.blue_cylinder_removed_segment`))
  (`/Engine/EditorBlueprintResources/StandardMacros.CompareInt` crystal_id (`self.crystal_id_to_hide_this`)
    (:`==`
      (`SceneComponent.SetVisibility` _blue_cylinder_removed_segment true false)
      (`PrimitiveComponent.SetMaterial` _blue_cylinder_removed_segment 0 "/Game/Materials/Transparent/MI_Blue_Transparent_2.MI_Blue_Transparent_2")
      (if (not (`self.IsFlashing`))
        (`FMODAudioComponent.Play` (`self.FMODDeactivatecrystal`))
        (set `self.IsFlashing` true)))))

(fn `UserConstructionScript`
  (`parent.UserConstructionScript`))