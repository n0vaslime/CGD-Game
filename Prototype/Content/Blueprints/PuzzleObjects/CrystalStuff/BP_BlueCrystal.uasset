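; Blue crystal puzzle object that, when hit, lights up and temporarily shows its linked objects through the BPI_Showable interface.
; Tick counts down the active time, blinks during the final fifth, then restores the base material and hides the objects on expiry.
; Each blink toggles the emissive material and alternates objects between shown and partially hidden.
; Calls pass CrystalId, except the blink's re-show, which passes 0.
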(event `self.ReceiveTick`
  (params (DeltaSeconds :type "Float (single-precision)"))
  (`self.updateTimers` DeltaSeconds))

(event `self.Hit`
  (params (Damage :type "Float (double-precision)") (Hitter :type "Actor Object Reference"))
  (`self.activateCrystal`))

(fn `activateCrystal`
  (`PrimitiveComponent.SetMaterial` (`self.CrystalMesh`) 0 "/Game/Materials/Crystal/M_CrystalLit.M_CrystalLit")
  (for _array_element (`self.ObjectsToShow`)
    (bind _asbpi_showable (cast `/Game/Interfaces/BPI_Showable` _array_element))
    (`/Game/Interfaces/BPI_Showable.show` _asbpi_showable (`self.crystal_id`)))
  (set `self.lit` true)
  (set `self.blink_timer` 0.0)
  (set `self.active_timer` (`self.time_active`))
  (set `self.lit` false))

(fn `blink`
  (bind _objectstoshow (`self.ObjectsToShow`))
  (if (`self.lit`)
    (`PrimitiveComponent.SetMaterial` (`self.CrystalMesh`) 0 "/Game/Materials/M_EmissiveTurquoise_2.M_EmissiveTurquoise_2")
    (set `self.lit` false)
    (for _array_element _objectstoshow
      (bind _asbpi_showable (cast `/Game/Interfaces/BPI_Showable` _array_element))
      (`/Game/Interfaces/BPI_Showable.partiallyHide` _asbpi_showable (`self.crystal_id`)))
    (else
      (`PrimitiveComponent.SetMaterial` (`self.CrystalMesh`) 0 "/Game/Materials/M_EmissiveTurquoise.M_EmissiveTurquoise")
      (set `self.lit` true)
      (for _array_element_2 _objectstoshow
        (bind _asbpi_showable_2 (cast `/Game/Interfaces/BPI_Showable` _array_element_2))
        (`/Game/Interfaces/BPI_Showable.show` _asbpi_showable_2 0)))))

(fn `deactivateCrystal`
  (`PrimitiveComponent.SetMaterial` (`self.CrystalMesh`) 0 "/Game/Materials/Crystal/M_CrystalBase.M_CrystalBase")
  (for _array_element (`self.ObjectsToShow`)
    (bind _asbpi_showable (cast `/Game/Interfaces/BPI_Showable` _array_element))
    (`/Game/Interfaces/BPI_Showable.hide` _asbpi_showable (`self.crystal_id`))))

(fn `updateTimers`
  (params (`Delta Seconds` :type "Float (double-precision)"))
  (bind _active_timer (`self.active_timer`))
  (`/Engine/EditorBlueprintResources/StandardMacros.CompareFloat` _active_timer
    (:`>`
      (`/Engine/EditorBlueprintResources/StandardMacros.CompareFloat` _active_timer (`self.blink_point`)
        (:`>`
          _)
        (:`==`
          (bind _output_get (set `self.blink_timer` (- (`self.blink_timer`) `Delta Seconds`) :!label _label))
          (`/Engine/EditorBlueprintResources/StandardMacros.CompareFloat` _output_get
            (:`>`
              _)
            (:`==`
              (`self.blink` :!label _label_2)
              (set `self.blink_timer` (`self.time_to_blink`)))
            (:`<`
              (goto _label_2))))
        (:`<`
          (goto _label)))
      (bind _output_get_2 (set `self.active_timer` (- _active_timer `Delta Seconds`)))
      (`/Engine/EditorBlueprintResources/StandardMacros.CompareFloat` _output_get_2
        (:`==`
          _)
        (:`<`
          _))
      (`self.deactivateCrystal`))))

(fn `UserConstructionScript`
  ;[0 1 1] Set Blink point (when crystal start blinking) based on time it will be active
  (set `self.blink_point` (* (`self.time_active`) 0.2)))