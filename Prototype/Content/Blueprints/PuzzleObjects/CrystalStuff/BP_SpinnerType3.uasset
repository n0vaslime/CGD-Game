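; BP_SpinnerType3 is a crystal puzzle object with three blue blocks that can be shown, hidden or partially hidden.
; Show makes them visible with a translucent material and stores any positive crystal ID; Hide and PartiallyHide act only on that ID.
; PartiallyHide swaps to a second transparent material as a flashing state.
; IsLit and IsFlashing flags stop the FMOD activate and deactivate sounds from retriggering.
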(event `/Game/Interfaces/BPI_Showable.show`
  (params (crystal_id :type Integer))
  (bind _block_001_blue (`self.block_001_blue`))
  (if (> crystal_id 0)
    (set `self.crystal_id_to_hide_this` crystal_id))
  (`SceneComponent.SetVisibility` _block_001_blue true false)
  (`SceneComponent.SetVisibility` (`self.block_002_blue`) true false)
  (`SceneComponent.SetVisibility` (`self.block_003_blue`) true false)
  (`PrimitiveComponent.SetMaterial` _block_001_blue 0 "/Game/Materials/Transparent/MI_TranslucentBlue.MI_TranslucentBlue")
  (`PrimitiveComponent.SetMaterial` (`self.block_002_blue`) 0 "/Game/Materials/Transparent/MI_TranslucentBlue.MI_TranslucentBlue")
  (`PrimitiveComponent.SetMaterial` (`self.block_003_blue`) 0 "/Game/Materials/Transparent/MI_TranslucentBlue.MI_TranslucentBlue")
  (if (not (`self.IsLit`))
    (`FMODAudioComponent.Play` (`self.FMODActivateCrystal`))
    (set `self.IsLit` true)))

(event `/Game/Interfaces/BPI_Showable.hide`
  (params (crystal_id :type Integer))
  (`/Engine/EditorBlueprintResources/StandardMacros.CompareInt` crystal_id (`self.crystal_id_to_hide_this`)
    (:`==`
      (`SceneComponent.SetVisibility` (`self.block_001_blue`) false false)
      (`SceneComponent.SetVisibility` (`self.block_002_blue`) false false)
      (`SceneComponent.SetVisibility` (`self.block_003_blue`) false false)
      (set `self.IsLit` false)
      (set `self.IsFlashing` false))))

(event `/Game/Interfaces/BPI_Showable.partiallyHide`
  (params (crystal_id :type Integer))
  (`/Engine/EditorBlueprintResources/StandardMacros.CompareInt` crystal_id (`self.crystal_id_to_hide_this`)
    (:`==`
      (`SceneComponent.SetVisibility` (`self.block_003_blue`) true false)
      (`SceneComponent.SetVisibility` (`self.block_002_blue`) true false)
      (`SceneComponent.SetVisibility` (`self.block_001_blue`) true false)
      (`PrimitiveComponent.SetMaterial` (`self.block_002_blue`) 0 "/Game/Materials/Transparent/MI_Blue_Transparent_2.MI_Blue_Transparent_2")
      (`PrimitiveComponent.SetMaterial` (`self.block_003_blue`) 0 "/Game/Materials/Transparent/MI_Blue_Transparent_2.MI_Blue_Transparent_2")
      (`PrimitiveComponent.SetMaterial` (`self.block_001_blue`) 0 "/Game/Materials/Transparent/MI_Blue_Transparent_2.MI_Blue_Transparent_2")
      (if (not (`self.IsFlashing`))
        (`FMODAudioComponent.Play` (`self.FMODDeactivatecrystal`))
        (set `self.IsFlashing` true)))))

(fn `UserConstructionScript`
  (`parent.UserConstructionScript`))