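; BP_CheckpointInvisible is a single-use invisible checkpoint that moves the player's respawn point.
; When a BP_ThirdPersonCharacter overlaps CheckpointCollidor, a CheckPointUsed flag ensures the update runs only once.
; It then finds player 0's pawn and passes the world location of the PlayerSpawnPosition marker to that pawn's BPC_DeathComponent via UpdateRespawnLocation.
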(event `self.CheckpointCollidor.OnComponentBeginOverlap`
  (params (OverlappedComponent :type "PrimitiveComponent Object Reference") (OtherActor :type "Actor Object Reference") (OtherComp :type "PrimitiveComponent Object Reference") (OtherBodyIndex :type Integer) (bFromSweep :type Boolean) (SweepResult :type "HitResult Structure (by ref)"))
  (cast `/Game/ThirdPerson/Blueprints/BP_ThirdPersonCharacter` OtherActor)
  ;[1 1 1] To make sure setting the bool isn't spammed multiple times
  (if (not (`self.CheckPointUsed`))
    (set `self.CheckPointUsed` true)
    ;[1 1 1] Update the player's respawn location with that of the position marker
    (bind _asbp_third_person_character (cast `/Game/ThirdPerson/Blueprints/BP_ThirdPersonCharacter` (`Controller.K2_GetPawn` (`PlayerState.GetPlayerController` (`GameplayStatics.GetPlayerState` 0)))))
    (`/Game/Blueprints/DeathSystem/BPC_DeathComponent.UpdateRespawnLocation` (`self.GetComponentByClass` _asbp_third_person_character "/Game/Blueprints/DeathSystem/BPC_DeathComponent.BPC_DeathComponent_C") (`SceneComponent.K2_GetComponentLocation` (`self.PlayerSpawnPosition`)))))

(fn `UserConstructionScript`)