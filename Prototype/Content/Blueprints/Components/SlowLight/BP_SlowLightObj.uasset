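; BP_SlowLightObj is a light volume that slows certain gameplay objects while they are inside it.
; LightCollision overlap begin casts the actor to a spinning platform, bullet or turret, lowering its speed or lengthening its shot cooldown.
; Overlap end writes back hardcoded normal values rather than the actor's previous ones.
; Logic to follow the third-person character's light arrow is disconnected, so BeginPlay and Tick do nothing.
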(event `self.ReceiveBeginPlay`
  ;[0.3284 1 0.3125] Gets Pos and Rot of arrow component in front of player
  ;;[1 1 1] Had to decouple for build safety
)

(event `self.ReceiveTick`
  (params (DeltaSeconds :type "Float (single-precision)"))
  ;[1 1 1] Had to decouple for build safety
)

(event `self.LightCollision.OnComponentBeginOverlap`
  (params (OverlappedComponent :type "PrimitiveComponent Object Reference") (OtherActor :type "Actor Object Reference") (OtherComp :type "PrimitiveComponent Object Reference") (OtherBodyIndex :type Integer) (bFromSweep :type Boolean) (SweepResult :type "HitResult Structure (by ref)"))
  (bind _asbp_spin_plat (cast `/Game/Blueprints/Objects/BP_SpinPlat` OtherActor)
    (:`then`
      (set `/Game/Blueprints/Objects/BP_SpinPlat.SpinPlatSpeed` 10.0 _asbp_spin_plat))
    (:`CastFailed`
      (bind _asbp_bullet (cast `/Game/Blueprints/Projectiles/BP_Bullet` OtherActor)
        (:`then`
          (set `/Game/Blueprints/Projectiles/BP_ProjectileParent.speed` 100.0 _asbp_bullet))
        (:`CastFailed`
          (bind _asbp_basic_turret (cast `/Game/Blueprints/Enemies/BP_BasicTurret` OtherActor))
          (set `/Game/Blueprints/Enemies/BP_TurretParent.max_shot_cooldown` 2.0 _asbp_basic_turret))))))

(event `self.LightCollision.OnComponentEndOverlap`
  (params (OverlappedComponent :type "PrimitiveComponent Object Reference") (OtherActor :type "Actor Object Reference") (OtherComp :type "PrimitiveComponent Object Reference") (OtherBodyIndex :type Integer))
  (bind _asbp_spin_plat (cast `/Game/Blueprints/Objects/BP_SpinPlat` OtherActor)
    (:`then`
      (set `/Game/Blueprints/Objects/BP_SpinPlat.SpinPlatSpeed` 90.0 _asbp_spin_plat))
    (:`CastFailed`
      (bind _asbp_bullet (cast `/Game/Blueprints/Projectiles/BP_Bullet` OtherActor)
        (:`then`
          (set `/Game/Blueprints/Projectiles/BP_ProjectileParent.speed` 1000.0 _asbp_bullet))
        (:`CastFailed`
          (bind _asbp_basic_turret (cast `/Game/Blueprints/Enemies/BP_BasicTurret` OtherActor))
          (set `/Game/Blueprints/Enemies/BP_TurretParent.max_shot_cooldown` 1.0 _asbp_basic_turret))))))

(fn `UserConstructionScript`)