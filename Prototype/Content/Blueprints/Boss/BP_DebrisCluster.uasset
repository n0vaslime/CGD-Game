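; BP_DebrisCluster is a falling debris hazard for the boss fight that kills the player on hitting their capsule.
; After a random delay it randomizes material and rotation, then line-traces down to spawn a warning shadow.
; Tick moves it down with a swept move until it lands with a sound, or destroys itself on hitting other debris.
; Laser hits and resets destroy it, and EnablePowerup flags it blue.
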(event `self.ReceiveBeginPlay`
  (bind _returnvalue (`KismetMathLibrary.RandomFloatInRange` -180.0 180.0))
  (bind _returnvalue_2 (`SceneComponent.K2_GetComponentLocation` (`self.Cube1`)))
  (`KismetSystemLibrary.Delay` (`KismetMathLibrary.RandomFloatInRange` 0.0 5.0))
  (set `self.started` true)
  (`PrimitiveComponent.SetMaterial` (`self.Cube`) 0 (`KismetArrayLibrary.Array_Random` (`self.mats`)))
  (`SceneComponent.K2_SetRelativeRotation` (`self.Cube`) (`KismetMathLibrary.MakeRotator` _returnvalue _returnvalue _returnvalue) false false)
  ;[1 1 1] Spawns shadow
  (bind _outhit (`KismetSystemLibrary.LineTraceSingleForObjects` _returnvalue_2 (- _returnvalue_2 (0.0 0.0 10000.0)) (`|MakeArray` "ObjectTypeQuery1" :!type "EObjectTypeQuery Enum")))
  (bind _returnvalue_3 (`|SpawnActorFromClass` "/Game/Blueprints/Boss/BP_DebrisShadow.BP_DebrisShadow_C" (`KismetMathLibrary.MakeTransform` (`.Location` (`GameplayStatics.BreakHitResult` _outhit)) (struct :`Yaw` 45.0)) "Undefined" "MultiplyWithRoot" null null))
  (set `self.shadow` _returnvalue_3))

(event `self.ReceiveTick`
  (params (DeltaSeconds :type "Float (single-precision)"))
  (if (`self.started`)
    ;[1 1 1] Moves debris down if not on floor
    (if (not (`self.landed`))
      (bind _sweephitresult (`self.K2_SetActorLocation` (+ (* (`self.Fallspeed`) DeltaSeconds) (`self.K2_GetActorLocation`)) true))
      (bind (_bblockinghit _binitialoverlap _time _distance _location _impactpoint _normal _impactnormal _physmat _hitactor _hitcomponent) (`GameplayStatics.BreakHitResult` _sweephitresult))
      (if _bblockinghit
        (bind _returnvalue (`GameplayStatics.GetObjectClass` _hitactor))
        (if (or (== _returnvalue "BP_DebrisCluster_C") (== _returnvalue "/Game/Blueprints/Boss/BP_FallingDebris.BP_FallingDebris_C"))
          (`self.K2_DestroyActor` (`self.shadow`))
          (`self.K2_DestroyActor`)
          (else
            ;[1 1 1] Kills the player if it hits them
            (bind _asbp_third_person_character (cast `/Game/ThirdPerson/Blueprints/BP_ThirdPersonCharacter` _hitactor)
              (:`then`
                (if (== (`Character.CapsuleComponent` _asbp_third_person_character) _hitcomponent)
                  (`/Game/Blueprints/DeathSystem/BPC_DeathComponent.Execute Death Sequence` (`/Game/ThirdPerson/Blueprints/BP_ThirdPersonCharacter.BPC_Death Component` _asbp_third_person_character))))
              (:`CastFailed`
                (set `self.landed` true)
                (`FMODAudioComponent.Play` (`self.FMODFallingDebrisSmall`))
                (`self.K2_DestroyActor` (`self.shadow`))))))))))

(event `self.LaserHit`
  (params (Location :type "Vector Structure") (Type :type "/Game/LaserType Structure"))
  ;[1 1 1] destroys when hit by boss laser
  (`self.Reset`))

(event `Reset`
  (bind _shadow (`self.shadow`))
  (if (`KismetSystemLibrary.IsValid` _shadow)
    (`self.K2_DestroyActor` _shadow))
  (`self.K2_DestroyActor`))

(fn `EnablePowerup`
  (`PrimitiveComponent.SetMaterial` (`self.Cube`) 0 "/Game/Materials/BasicColours/M_Blue.M_Blue")
  (set `self.IsPowerup` true))

(fn `UserConstructionScript`)