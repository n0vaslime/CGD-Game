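; Boss-fight falling debris that spawns above the player with a randomized look and a traced ground shadow.
; Tick sweeps it down, killing the player on capsule hits and resolving debris collisions in favor of powerup or empowered pieces.
; EnablePowerup makes a small glowing piece that becomes a BP_ReinforceHammer on landing.
; Empower makes a larger, slower piece over a random BP_SpawnCluster that lands as a shockwave and ignores lasers.
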(event `self.ReceiveBeginPlay`
  (bind _returnvalue (`KismetMathLibrary.RandomFloatInRange` -180.0 180.0))
  ;[1 1 1] Spawns above the player
  (`PrimitiveComponent.SetMaterial` (`self.Cube`) 0 (`KismetArrayLibrary.Array_Random` (`self.mats`)))
  (`SceneComponent.K2_SetRelativeRotation` (`self.Cube`) (`KismetMathLibrary.MakeRotator` _returnvalue _returnvalue _returnvalue) false false)
  (bind _returnvalue_2 (`GameplayStatics.GetActorOfClass` "/Game/ThirdPerson/Blueprints/BP_ThirdPersonCharacter.BP_ThirdPersonCharacter_C"))
  (bind (_returnvalue_x _returnvalue_y _returnvalue_z) (`KismetMathLibrary.BreakVector` (`self.K2_GetActorLocation` _returnvalue_2)))
  (bind _returnvalue_3 (`KismetMathLibrary.MakeVector` _returnvalue_x _returnvalue_y (+ _returnvalue_z 2000.0)))
  (`self.K2_SetActorLocation` _returnvalue_3)
  ;[1 1 1] Spawns shadow
  (bind _outhit (`KismetSystemLibrary.LineTraceSingleForObjects` _returnvalue_3 (- _returnvalue_3 (0.0 0.0 10000.0)) (`|MakeArray` "ObjectTypeQuery1" :!type "EObjectTypeQuery Enum")))
  (bind _returnvalue_4 (`|SpawnActorFromClass` "/Game/Blueprints/Boss/BP_DebrisShadow.BP_DebrisShadow_C" (`KismetMathLibrary.MakeTransform` (`.Location` (`GameplayStatics.BreakHitResult` _outhit)) (struct :`Yaw` 45.0)) "Undefined" "MultiplyWithRoot" null null))
  (set `self.shadow` _returnvalue_4))

(event `self.ReceiveTick`
  (params (DeltaSeconds :type "Float (single-precision)"))
  ;[1 1 1] Moves debris down if not on floor
  (if (not (`self.landed`))
    (bind _sweephitresult (`self.K2_SetActorLocation` (+ (* (`self.Fallspeed`) DeltaSeconds (`self.fallspeed multiplier`)) (`self.K2_GetActorLocation`)) true))
    (bind (_bblockinghit _binitialoverlap _time _distance _location _impactpoint _normal _impactnormal _physmat _hitactor _hitcomponent) (`GameplayStatics.BreakHitResult` _sweephitresult))
    (if _bblockinghit
      (bind _returnvalue (`GameplayStatics.GetObjectClass` _hitactor))
      ;[1 1 1] Destroys the appropriate debris if 2 collide (prioritises keeping blue debris)
      (if (or (== _returnvalue "/Game/Blueprints/Boss/BP_DebrisCluster.BP_DebrisCluster_C") (== _returnvalue "BP_FallingDebris_C"))
        (if (or (`self.IsPowerup`) (`self.empowered`))
          (`self.K2_DestroyActor` _hitactor)
          (else
            (`self.K2_DestroyActor` (`self.shadow`))
            (`self.K2_DestroyActor`)))
        (else
          ;[1 1 1] Kills the player if it hits them
          (bind _asbp_third_person_character (cast `/Game/ThirdPerson/Blueprints/BP_ThirdPersonCharacter` _hitactor)
            (:`then`
              (if (and (== (`Character.CapsuleComponent` _asbp_third_person_character) _hitcomponent) (not (`self.IsPowerup`)))
                (`/Game/Blueprints/DeathSystem/BPC_DeathComponent.Execute Death Sequence` (`/Game/ThirdPerson/Blueprints/BP_ThirdPersonCharacter.BPC_Death Component` _asbp_third_person_character))
                (`FMODAudioComponent.Play` (`/Game/ThirdPerson/Blueprints/BP_ThirdPersonCharacter.FMODDeath` _asbp_third_person_character))))
            (:`CastFailed`
              (set `self.landed` true)
              (`FMODAudioComponent.Play` (`self.FMODFallingDebrisSmall`))
              (`self.K2_DestroyActor` (`self.shadow`))
              (if (`self.empowered`)
                ;[1 1 1] Spawn Shockwave
                (`|SpawnActorFromClass` "/Game/Blueprints/Boss/Shockwave/BP_Shockwave.BP_Shockwave_C" (`KismetMathLibrary.MakeTransform` (`SceneComponent.K2_GetComponentLocation` (`self.crystal spawn`))) "Undefined" "MultiplyWithRoot" null null)
                (`self.K2_DestroyActor`)
                (else
                  ;[1 1 1] Spawns a powerup if blue
                  (if (`self.IsPowerup`)
                    (`|SpawnActorFromClass` "/Game/Blueprints/PuzzleObjects/BP_ReinforceHammer.BP_ReinforceHammer_C" (`KismetMathLibrary.MakeTransform` (`self.K2_GetActorLocation`)) "Undefined" "MultiplyWithRoot" null null)
                    (`self.K2_DestroyActor`)))))))))))

(event `/Game/Interfaces/BPI_LaserInteractable.LaserHit`
  (params (Location :type "Vector Structure") (Type :type "/Game/LaserType Structure"))
  ;[1 1 1] destroys when hit by boss laser
  (if (not (`self.empowered`))
    (`self.Reset`)))

(event `empower`
  (bind (_returnvalue_x _returnvalue_y _returnvalue_z) (`KismetMathLibrary.BreakVector` (`self.K2_GetActorLocation`)))
  (bind _shadow (`self.shadow`))
  (bind (_returnvalue_x_2 _returnvalue_y_2 _returnvalue_z_2) (`KismetMathLibrary.BreakVector` (`self.K2_GetActorLocation` _shadow)))
  (set `self.Fallspeed` (* (`self.Fallspeed`) 0.8))
  (set `self.empowered` true)
  (`self.SetActorScale3D` (* (`self.GetActorScale3D`) 2.0))
  (`self.SetActorScale3D` (`self.shadow`) (2.0 2.0 2.0))
  (bind _outactors (`GameplayStatics.GetAllActorsOfClass` "/Game/Blueprints/Boss/BP_SpawnCluster.BP_SpawnCluster_C"))
  (bind _output_get (set `self.spawn` (`|GetArrayItem` _outactors (`KismetMathLibrary.RandomInteger` (`KismetArrayLibrary.Array_Length` _outactors)))))
  (bind (_returnvalue_x_3 _returnvalue_y_3) (`KismetMathLibrary.BreakVector` (`self.K2_GetActorLocation` _output_get)))
  (`self.K2_SetActorLocation` (`KismetMathLibrary.MakeVector` _returnvalue_x_3 _returnvalue_y_3 _returnvalue_z))
  (`self.K2_SetActorLocation` _shadow (`KismetMathLibrary.MakeVector` _returnvalue_x_3 _returnvalue_y_3 _returnvalue_z_2) false false))

(event `Reset`
  (bind _shadow (`self.shadow`))
  (if (`KismetSystemLibrary.IsValid` _shadow)
    (`self.K2_DestroyActor` _shadow))
  (`self.K2_DestroyActor`))

(fn `EnablePowerup`
  (bind _shadow (`self.shadow`))
  (`PrimitiveComponent.SetMaterial` (`self.Cube`) 0 "/Game/Materials/Glow/Glow.Glow")
  (set `self.IsPowerup` true)
  (`self.SetActorScale3D` (* (`self.GetActorScale3D`) 0.6))
  (`self.SetActorScale3D` _shadow (* (`self.GetActorScale3D` _shadow) 0.6))
  (`SceneComponent.K2_AddLocalOffset` (`self.Cube`) (0.0 0.0 100.0) false false)
  (`PrimitiveComponent.SetCollisionResponseToChannel` (`self.Cube1`) "ECC_Pawn" "ECR_Ignore"))

(fn `UserConstructionScript`)