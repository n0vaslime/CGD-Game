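; BP_CliffCharacter is the Cliff character visual, which plays a hammer slam montage based on the player's hit state.
; BeginPlay caches the third-person player, and Tick polls its CanHit flag, playing the slam on SkCliff while that flag is false.
; An AnimPlay gate blocks restarts until the montage completes.
; A separate PlayHammerSlamAnimation function plays the same montage directly, without the gate.
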(event `self.ReceiveBeginPlay`
  (bind _asbp_third_person_character (cast `/Game/ThirdPerson/Blueprints/BP_ThirdPersonCharacter` (`GameplayStatics.GetPlayerCharacter` 0)))
  (set `self.PlayerReference` _asbp_third_person_character))

(event `self.ReceiveTick`
  (params (DeltaSeconds :type "Float (single-precision)"))
  (if (`/Game/ThirdPerson/Blueprints/BP_ThirdPersonCharacter.Can Hit` (`self.PlayerReference`))
    _
    (elif (`self.AnimPlay`)
      (set `self.AnimPlay` false)
      (`|PlayMontage` (`self.sk-Cliff`) "/Game/ART+VISUALS/AnimationFolder/AM_Hammer_Slam_Anim.AM_Hammer_Slam_Anim"
        (:`OnCompleted`
          (set `self.AnimPlay` true))))))

(fn `Play Hammer Slam Animation`
  (`AnimInstance.Montage_Play` (`SkeletalMeshComponent.GetAnimInstance` (`self.sk-Cliff`)) "/Game/ART+VISUALS/AnimationFolder/AM_Hammer_Slam_Anim.AM_Hammer_Slam_Anim" 1.0 "MontageLength" 0.0 true))

(fn `UserConstructionScript`)